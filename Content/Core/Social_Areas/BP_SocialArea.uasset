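; BP_SocialArea is a box-volume social area that tracks how many BP_coworkers are inside it.
; It recounts overlapping coworkers shortly after BeginPlay and on every begin and end overlap.
; It calls ExitAreaMessage on the overlapping actor when more than one coworker is inside on entry, or when any remain on exit.
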(event `self.ReceiveBeginPlay`
  (`KismetSystemLibrary.Delay` 0.2)
  (`self.CountPeopleInsideArea`))

(event `self.Box.OnComponentBeginOverlap`
  (params (OverlappedComponent :type "PrimitiveComponent Object Reference") (OtherActor :type "Actor Object Reference") (OtherComp :type "PrimitiveComponent Object Reference") (OtherBodyIndex :type Integer) (bFromSweep :type Boolean) (SweepResult :type "HitResult Structure (by ref)"))
  (`self.CountPeopleInsideArea`)
  (if (> (`self.PeopleInside`) 1)
    (message `/Game/Core/coworkers/BPI_ExitAreaWithCoworkers.ExitArea` OtherActor)))

(event `self.Box.OnComponentEndOverlap`
  (params (OverlappedComponent :type "PrimitiveComponent Object Reference") (OtherActor :type "Actor Object Reference") (OtherComp :type "PrimitiveComponent Object Reference") (OtherBodyIndex :type Integer))
  (`self.CountPeopleInsideArea`)
  (if (> (`self.PeopleInside`) 0)
    (message `/Game/Core/coworkers/BPI_ExitAreaWithCoworkers.ExitArea` OtherActor)))

(fn `CountPeopleInsideArea`
  (set `self.PeopleInside` 0)
  (for _ (`PrimitiveComponent.GetOverlappingActors` (`self.Box`) "/Game/Core/coworkers/BP_coworkers.BP_coworkers_C")
    (`/Engine/EditorBlueprintResources/StandardMacros.IncrementInt` (`self.PeopleInside`))))

(fn `UserConstructionScript`)